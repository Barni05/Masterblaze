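; AI controller for guard NPCs that starts the guard blackboard and behavior tree on BeginPlay.
; When perception senses an actor without the "Enemy" tag, it stores the player pawn as the enemy key and starts a looping fire timer.
; Losing that stimulus clears both.
; Tick caches the controlled NPC character and drives its aiming and shooting flags from whether a focus actor exists.
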(event `self.ReceiveBeginPlay`
  (bind _asnpcaicontroller (cast `NPCAIController` self))
  (bind _blackboardcomponent (`self.UseBlackboard` _asnpcaicontroller "/Game/Dynamic/TPS/NPC/NPCBehaviour/GuardData.GuardData"))
  (set `self.BlackboardComp` _blackboardcomponent)
  (`self.RunBehaviorTree` _asnpcaicontroller "/Game/Dynamic/TPS/NPC/NPCBehaviour/GuardBehaviour.GuardBehaviour"))

(event `self.AIPerception.OnTargetPerceptionUpdated`
  (params (Actor :type "Actor Object Reference") (Stimulus :type "AIStimulus Structure"))
  (if (`self.ActorHasTag` Actor "Enemy")
    _
    (elif Stimulus_bSuccessfullySensed
      (`BlackboardComponent.SetValueAsObject` (`self.BlackboardComp`) (`self.EnemyKey`) (`GameplayStatics.GetPlayerPawn` 0))
      (bind _returnvalue (`KismetSystemLibrary.K2_SetTimerDelegate` (delegate `FireExpired`) 1.0 true))
      (else
        (`BlackboardComponent.ClearValue` (`self.BlackboardComp`) (`self.EnemyKey`))
        (`KismetSystemLibrary.K2_ClearAndInvalidateTimerHandle` _returnvalue)))))

(event `FireExpired`
  (`/Game/Dynamic/TPS/NPC/NPCBehaviour/NPCCaharacter_BP.Fire` (stale `self.ReceiveTick` _asnpccaharacter_bp)))

(event `self.ReceiveTick`
  (params (DeltaSeconds :type "Float (single-precision)"))
  (bind _returnvalue (`KismetSystemLibrary.IsValid` (`self.GetFocusActor`)))
  (bind _asnpccaharacter_bp (cast `/Game/Dynamic/TPS/NPC/NPCBehaviour/NPCCaharacter_BP` (`self.K2_GetPawn`)))
  (set `/Game/Dynamic/TPS/NPC/NPCBehaviour/NPCCaharacter_BP.Aiming` _returnvalue _asnpccaharacter_bp)
  (set `/Game/Dynamic/TPS/NPC/NPCBehaviour/NPCCaharacter_BP.Shooting` _returnvalue _asnpccaharacter_bp))

(fn `UserConstructionScript`)