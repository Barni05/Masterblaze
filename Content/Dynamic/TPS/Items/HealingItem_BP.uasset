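; HealingItem_BP is a spinning health pickup that heals the player on overlap and then destroys itself.
; Tick rotates it in yaw at RotatePerSecond.
; On overlap, it scans the Box's overlapping actors for the Player tag, then casts player pawn 0 to Player_BP.
; If Health is below the hardcoded cap, it prints a debug message and adds a fixed amount without clamping the result.
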(event `self.ReceiveTick`
  (params (DeltaSeconds :type "Float (single-precision)"))
  (`self.K2_AddActorWorldRotation` (`KismetMathLibrary.MakeRotator` 0.0 0.0 (* DeltaSeconds (`self.RotatePerSecond`)))))

(event `self.ReceiveActorBeginOverlap`
  (params (OtherActor :type "Actor Object Reference"))
  (for _array_element (`PrimitiveComponent.GetOverlappingActors` (`self.Box`) null)
    (if (`self.ActorHasTag` _array_element "Player")
      (bind _asplayer_bp (cast `/Game/Dynamic/TPS/Behaviour/Player_BP` (`GameplayStatics.GetPlayerPawn` 0)))
      (bind _health (`/Game/Dynamic/TPS/Behaviour/Player_BP.Health` _asplayer_bp))
      (if (< _health 100.0)
        (`KismetSystemLibrary.PrintString` "has low hp")
        (set `/Game/Dynamic/TPS/Behaviour/Player_BP.Health` (+ _health 20.0) _asplayer_bp)
        (`self.K2_DestroyActor`)))))

(fn `UserConstructionScript`)