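; BP_HealingItem is a rotating health pickup that heals the player on contact.
; Tick spins the Item component around yaw by RotationSpeed each frame, without scaling by delta time.
; When an actor tagged Player overlaps Bound, it casts to Player_BP, adds a fixed amount to Health and destroys itself.
; A clamp node for Health is left unconnected, so the pickup applies no upper limit.
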(event `self.ReceiveTick`
  (params (DeltaSeconds :type "Float (single-precision)"))
  (`SceneComponent.K2_AddWorldRotation` (`self.Item`) (`KismetMathLibrary.MakeRotator` 0.0 0.0 (`self.RotationSpeed`)) false false))

(event `self.Bound.OnComponentBeginOverlap`
  (params (OverlappedComponent :type "PrimitiveComponent Object Reference") (OtherActor :type "Actor Object Reference") (OtherComp :type "PrimitiveComponent Object Reference") (OtherBodyIndex :type Integer) (bFromSweep :type Boolean) (SweepResult :type "HitResult Structure (by ref)"))
  (set `self.OverlappedActor` OtherActor)
  (if (`self.ActorHasTag` OtherActor "Player")
    (bind _asplayer_bp (cast `/Game/Dynamic/TPS/Behaviour/Player_BP` (`self.OverlappedActor`)))
    (bind _output_get (set `/Game/Dynamic/TPS/Behaviour/Player_BP.Health` (+ (`/Game/Dynamic/TPS/Behaviour/Player_BP.Health` _asplayer_bp) 20.0) _asplayer_bp))
    (`self.K2_DestroyActor`)))

(fn `UserConstructionScript`)